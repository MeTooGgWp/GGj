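; BP_GlideOnMalus is a malus pickup that triggers a glide penalty when a flower touches it.
; When its collision overlaps a BP_Flower, it calls Glide on the GM_RopePuller game mode with MalusDuration, then destroys itself.
; The glide effect itself lives in the game mode, and the construction script only calls its parent.
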(event OnComponentBeginOverlap(Collision)
  (params (OverlappedComponent :type Primitive%20Component%20Object%20Reference) (OtherActor :type Actor%20Object%20Reference) (OtherComp :type Primitive%20Component%20Object%20Reference) (OtherBodyIndex :type Integer) (bFromSweep :type Boolean) (SweepResult :type Hit%20Result%20Structure%20%28by%20ref%29))
  (if (.bSuccess (Utilities|Casting|CastToBP_Flower OtherActor))
    (Default|Glide (.AsGM%20Rope%20Puller (Utilities|Casting|CastToGM_RopePuller (Game|GetGameMode))) (Variables|Default|GetmalusDuration))
    (Actor|DestroyActor)))

(event EventBeginPlay
  (|CallParentFunction) ; This node is disabled and will not be called.\nDrag off pins to build functionality.
)

(event Collision|EventActorBeginOverlap
  (params (OtherActor :type Actor%20Object%20Reference)))

(fn ConstructionScript
  (|CallParentFunction))