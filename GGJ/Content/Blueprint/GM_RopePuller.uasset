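; Game mode for a rope-puller game where the player loses if the light is too bright or too dark.
; UpdateIntensity adjusts a clamped LightIntensity, where low means bright and burns RopeStatus on Tick until defeat.
; High values play the ShadowAdvance timeline, scaled to TimeToShadowKill, moving a shadow hand toward defeat; mid-range values reverse it.
; Defeat pauses the game and shows the lose screen.
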(event Custom|defeatSequence
  (bind _returnvalue (Game|GetPlayerController 0))
  (Game|SetGamePaused true)
  (bind _returnvalue_2 (UserInterface|CreateWidget "/Game/Blueprint/Widget/W_LoseScreen.W_LoseScreen_C" _returnvalue))
  (UserInterface|Viewport|AddtoViewport _returnvalue_2 0)
  (Variables|/Script/Engine.PlayerController|SetbShowMouseCursor _returnvalue true)
  (Input|SetInputModeUIOnly _returnvalue _returnvalue_2 "LockOnCapture"))

(event Custom|checkDefeat
  ;[1 1 1] Check defeat condition
  (if (<= (Variables|Default|GetropeStatus) 0.0)
    (CallFunction|DefeatSequence)))

(event EventTick
  (params (DeltaSeconds :type Float%20%28single-precision%29))
  ;[1 1 1] If the player is too light
  (if (<= (Variables|Default|GetlightIntensity) 5.0)
    ;[1 1 1] Burn the rope
    (bind _output_get (Variables|Default|SetropeStatus (- (Variables|Default|GetropeStatus) (* DeltaSeconds (Variables|Default|GetBurningSpeed)))))
    ;[0.9117 1 0] Debug
    (Development|PrintString (Utilities|String|ToString(Float) _output_get))
    (CallFunction|CheckDefeat)
    (elif (>= (Variables|Default|GetlightIntensity) 95.0) ; If the player is too dark
      ;[1 1 1] Move shadow hand to snip players' rope
      (Utilities|FlowControl|DoOnce false :!label _label
        (:Completed
          (bind _newtrack_0 (Timeline|ShadowAdvance Play)
            (:Update
              (if (== _newtrack_0 1.0)
                (CallFunction|DefeatSequence)
                (else
                  (Variables|Default|SethandLocationRatio _newtrack_0)))))))
      (else
        (Utilities|FlowControl|Sequence
          (:then_0
            (goto _label Reset))
          (:then_1
            (Timeline|ShadowAdvance Reverse)))))))

(event EventBeginPlay
  ;[1 1 1] Initiate timeline to match time to kill
  (Components|Timeline|SetPlayRate (Variables|Default|GetShadowAdvance) (/ 1.0 (Variables|Default|GettimeToShadowKill))))

(fn ConstructionScript)

(fn UpdateIntensity
  (params (increasing? :type Boolean))
  (bind _returnvalue (Utilities|Time|GetWorldDeltaSeconds))
  (bind _lightvariation (Variables|Default|GetlightVariation))
  (bind _returnvalue_2 (* _lightvariation _returnvalue))
  (if increasing?
    ;[1 1 1] Check that the value is contain between 0-100
    (Variables|Default|SetlightIntensity (Math|Float|Clamp(Float) (- (Variables|Default|GetlightIntensity) _returnvalue_2) 0.0 1e+02))
    (else
      (Variables|Default|SetlightIntensity (Math|Float|Clamp(Float) (+ (Variables|Default|GetlightIntensity) _returnvalue_2) 0.0 1e+02)))))