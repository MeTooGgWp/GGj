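; BP_Flower is a flower that tracks a petal count and routes collected orbs to the two players.
; Petals increment with a debug print and decrement no lower than zero.
; The first basic orb sets a waiting flag, never cleared here; later ones make a random player absorb a shard.
; Shadow and light orbs set HasCharge on the matching character, found by casting player pawn 0, else using pawn 1.
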(fn ConstructionScript)

(fn AddPetal
  (Variables|Default|SetamountOfPetals (+ (Variables|Default|GetamountOfPetals) 1))
  (Development|PrintString "Petal Added"))

(fn RemovePetal
  (if (> (Variables|Default|GetamountOfPetals) 0)
    (Variables|Default|SetamountOfPetals (- (Variables|Default|GetamountOfPetals) 1))))

(fn CollectBasicOrbs
  (if (Variables|Default|GethasOrbsWaiting?)
    ;[1 1 1] randomly assign previous orb to a player
    (Default|AbsorbShard (.AsBP%20Player%20Lutin (Utilities|Casting|CastToBP_PlayerLutin (Game|Player|GetPlayerPawn (Math|Random|RandomInteger 2)))))
    (else
      ;[1 1 1] Assign Orbs to Flower
      (Variables|Default|SethasOrbsWaiting? true))))

(fn CollectShadowOrb
  (bind _returnvalue (Game|Player|GetPlayerPawn 0))
  (bind (_asbp_shadow_player _bsuccess) (Utilities|Casting|CastToBP_ShadowPlayer _returnvalue))
  ;[1 1 1] Determine wich player incarn the shadow character
  (if _bsuccess
    ;[1 1 1] Add charge if there was none
    (Variables|/Game/Blueprint/BP_PlayerLutin.BP_PlayerLutin_C|SethasCharge? _asbp_shadow_player true)
    (else
      (Variables|/Game/Blueprint/BP_PlayerLutin.BP_PlayerLutin_C|SethasCharge? (.AsBP%20Shadow%20Player (Utilities|Casting|CastToBP_ShadowPlayer (Game|Player|GetPlayerPawn 1))) true))))

(fn CollectLightOrb
  (bind _returnvalue (Game|Player|GetPlayerPawn 0))
  (bind (_asbp_light_player _bsuccess) (Utilities|Casting|CastToBP_LightPlayer _returnvalue))
  ;[1 1 1] Determine wich player incarn the light character
  (if _bsuccess
    ;[1 1 1] Add charge if there was none
    (Variables|/Game/Blueprint/BP_PlayerLutin.BP_PlayerLutin_C|SethasCharge? _asbp_light_player true)
    (else
      (Variables|/Game/Blueprint/BP_PlayerLutin.BP_PlayerLutin_C|SethasCharge? (.AsBP%20Light%20Player (Utilities|Casting|CastToBP_LightPlayer (Game|Player|GetPlayerPawn 1))) true))))