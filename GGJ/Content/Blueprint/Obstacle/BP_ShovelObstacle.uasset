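; BP_ShovelObstacle is a falling shovel hazard that damages the rope when it hits the flower.
; On BeginPlay it records its spawn location, and a timeline lerps the root straight down to a fixed Z without sweeping, simulating a fall.
; When its Box overlaps a BP_Flower, it tells GM_RopePuller to apply rope damage and check for defeat, then destroys itself.
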(event OnComponentBeginOverlap(Box)
  (params (OverlappedComponent :type Primitive%20Component%20Object%20Reference) (OtherActor :type Actor%20Object%20Reference) (OtherComp :type Primitive%20Component%20Object%20Reference) (OtherBodyIndex :type Integer) (bFromSweep :type Boolean) (SweepResult :type Hit%20Result%20Structure%20%28by%20ref%29))
  (bind _returnvalue (Game|GetGameMode))
  (bind _asgm_rope_puller (Utilities|Casting|CastToGM_RopePuller _returnvalue))
  ;[1 1 1] Dommage rope on hit
  (if (.bSuccess (Utilities|Casting|CastToBP_Flower OtherActor)) ; Check collision wit flower
    (Default|TakeRopeDommage _asgm_rope_puller)
    (Default|CheckDefeat _asgm_rope_puller)
    (Actor|DestroyActor)))

(event EventBeginPlay
  ;[1 1 1] Basic behaviour (simulate falling)
  (Variables|Default|SetinitialSpawnLocation (Transformation|GetActorLocation))
  (bind _newtrack_0 (Timeline|Timeline_0 PlayFromStart)
    (:Update
      (Transformation|SetWorldLocation (Variables|Transformation|GetRootComponent) (Math|Vector|Lerp(Vector) (Variables|Default|GetinitialSpawnLocation) (Math|Vector|MakeVector (.X (Math|Vector|BreakVector (Variables|Default|GetinitialSpawnLocation))) (.Y (Math|Vector|BreakVector (Variables|Default|GetinitialSpawnLocation))) -5e+02) _newtrack_0) false false))))

(fn ConstructionScript)