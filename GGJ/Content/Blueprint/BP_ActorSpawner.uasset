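; Spawner that repeatedly drops random obstacles, water drops, acid drops and orbs along the Y axis around its BoxArea.
; BeginPlay starts an endless delayed loop, each pass spawning a small random batch picked by weighted roll, mostly obstacles.
; GM_RopePuller's LightIntensity steers results: at extremes water and acid drops are forced to opposite Y signs.
; The rare special orb is Shadow at high intensity, Light otherwise.
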(event Custom|Relay
  (bind _returnvalue (Game|GetGameMode))
  (bind _returnvalue_2 (Game|GetGameMode))
  (bind _boxarea (Variables|Default|GetBoxArea))
  (bind _returnvalue_3 (Transformation|GetWorldLocation _boxarea))
  (bind _asgm_rope_puller (Utilities|Casting|CastToGM_RopePuller _returnvalue))
  (bind _asgm_rope_puller_2 (Utilities|Casting|CastToGM_RopePuller _returnvalue_2))
  (bind _boxextent (Variables|/Script/Engine.BoxComponent|GetBoxExtent _boxarea))
  (bind (_x _y _z) (Math|Vector|BreakVector _returnvalue_3))
  (bind _y_2 (Math|Vector|BreakVector _boxextent))
  (bind _lightintensity (Variables|/Game/Blueprint/GM_RopePuller.GM_RopePuller_C|GetlightIntensity _asgm_rope_puller))
  (bind _lightintensity_2 (Variables|/Game/Blueprint/GM_RopePuller.GM_RopePuller_C|GetlightIntensity _asgm_rope_puller_2))
  ;[1 1 1] To tweak on spawnrates and amount
  (Utilities|FlowControl|Delay (Variables|Default|GetSpawnDelay))
  (for _index (range 0 (Math|Random|RandomInteger 4))
    (if true ; determine if smth is spawn on this iteration
      (bind _output_get (Variables|Default|SetratioRandom (Math|Random|RandomFloatinRange 0.0 1.0)))
      (Variables|Default|SetrandomSpawnLocation (Math|Vector|MakeVector _x (+ _y (* 5 (Math|Random|RandomFloatinRange (* -100 _y_2) (* 100 _y_2)))) _z))
      (if (< _output_get 0.6) ; Check if spawn Obstacle
        (Game|SpawnActorfromClass "/Game/Blueprint/BP_TestObstacle.BP_TestObstacle_C" (Math|Transform|MakeTransform (Variables|Default|GetrandomSpawnLocation)) "DontSpawnIfColliding" 0 0)
        (else
          ;[0 0.7961 0.9062] WaterDrops
          (if (< (Variables|Default|GetratioRandom) 0.7) ; Check if spawn WaterDrop
            (if (or (> _lightintensity_2 75.0) (< _lightintensity_2 25.0)) ; Need to spawn in danger ?
              ;;[0 0.006305 0.1302] Control (The waterdrop will spawn in the more dangerous zone)
              (if (> _lightintensity_2 5e+01) ; side check
                ;;;[1 1 1] Obscurity
                (Game|SpawnActorfromClass "/Game/Blueprint/BP_WaterDrops.BP_WaterDrops_C" (Math|Transform|MakeTransform (Math|Vector|MakeVector (.X (Math|Vector|BreakVector (Variables|Default|GetrandomSpawnLocation))) (Math|Float|Absolute(Float) (.Y (Math|Vector|BreakVector (Variables|Default|GetrandomSpawnLocation)))) (.Z (Math|Vector|BreakVector (Variables|Default|GetrandomSpawnLocation))))) "Undefined" 0 0)
                (else
                  (Game|SpawnActorfromClass "/Game/Blueprint/BP_WaterDrops.BP_WaterDrops_C" (Math|Transform|MakeTransform (Math|Vector|MakeVector (.X (Math|Vector|BreakVector (Variables|Default|GetrandomSpawnLocation))) (* (Math|Float|Absolute(Float) (.Y (Math|Vector|BreakVector (Variables|Default|GetrandomSpawnLocation)))) -1.0) (.Z (Math|Vector|BreakVector (Variables|Default|GetrandomSpawnLocation))))) "Undefined" 0 0)))
              (else
                ;;[1 1 1] Spawn anywhere randomly
                (Game|SpawnActorfromClass "/Game/Blueprint/BP_WaterDrops.BP_WaterDrops_C" (Math|Transform|MakeTransform (Variables|Default|GetrandomSpawnLocation)) "Undefined" 0 0)))
            (else
              ;[0 1 0.05731] Acid Drops
              (if (< (Variables|Default|GetratioRandom) 0.8) ; Acid Drops
                (if (or (> _lightintensity 75.0) (< _lightintensity 25.0)) ; Need to spawn in danger ?
                  ;;[0 0 0] Control (The waterdrop will spawn in the more dangerous zone)
                  (if (> _lightintensity 5e+01) ; side check
                    ;;;[1 1 1] Obscurity
                    (Game|SpawnActorfromClass "/Game/Blueprint/BP_AcidDrops.BP_AcidDrops_C" (Math|Transform|MakeTransform (Math|Vector|MakeVector (.X (Math|Vector|BreakVector (Variables|Default|GetrandomSpawnLocation))) (* (Math|Float|Absolute(Float) (.Y (Math|Vector|BreakVector (Variables|Default|GetrandomSpawnLocation)))) -1.0) (.Z (Math|Vector|BreakVector (Variables|Default|GetrandomSpawnLocation))))) "Undefined" 0 0)
                    (else
                      (Game|SpawnActorfromClass "/Game/Blueprint/BP_AcidDrops.BP_AcidDrops_C" (Math|Transform|MakeTransform (Math|Vector|MakeVector (.X (Math|Vector|BreakVector (Variables|Default|GetrandomSpawnLocation))) (Math|Float|Absolute(Float) (.Y (Math|Vector|BreakVector (Variables|Default|GetrandomSpawnLocation)))) (.Z (Math|Vector|BreakVector (Variables|Default|GetrandomSpawnLocation))))) "Undefined" 0 0)))
                  (else
                    ;;[1 1 1] Spawn anywhere randomly
                    (Game|SpawnActorfromClass "/Game/Blueprint/BP_AcidDrops.BP_AcidDrops_C" (Math|Transform|MakeTransform (Variables|Default|GetrandomSpawnLocation)) "Undefined" 0 0)))
                (elif (< (Variables|Default|GetratioRandom) 0.95) ; Orbs : \nTrue = default\nFalse = timed orbs
                  ;[1 1 1] Basic orb
                  (Game|SpawnActorfromClass "/Game/Blueprint/BP_NormalOrb.BP_NormalOrb_C" (Math|Transform|MakeTransform (Variables|Default|GetrandomSpawnLocation)) "DontSpawnIfColliding" 0 0)
                  (else
                    ;[1 1 1] Specfic orb depending on light intensity
                    (if (> (Variables|/Game/Blueprint/GM_RopePuller.GM_RopePuller_C|GetlightIntensity (.AsGM%20Rope%20Puller (Utilities|Casting|CastToGM_RopePuller (Game|GetGameMode)))) 5e+01) ; Check light status
                      (Game|SpawnActorfromClass "/Game/Blueprint/BP_ShadowOrb.BP_ShadowOrb_C" (Math|Transform|MakeTransform (Variables|Default|GetrandomSpawnLocation)) "DontSpawnIfColliding" 0 0)
                      (else
                        (Game|SpawnActorfromClass "/Game/Blueprint/BP_LightOrb.BP_LightOrb_C" (Math|Transform|MakeTransform (Variables|Default|GetrandomSpawnLocation)) "DontSpawnIfColliding" 0 0))))))))))))
  (CallFunction|Relay))

(event EventBeginPlay
  (bind _returnvalue (Game|GetGameMode))
  (bind _returnvalue_2 (Game|GetGameMode))
  (bind _boxarea (Variables|Default|GetBoxArea))
  (bind _returnvalue_3 (Transformation|GetWorldLocation _boxarea))
  (bind _asgm_rope_puller (Utilities|Casting|CastToGM_RopePuller _returnvalue))
  (bind _asgm_rope_puller_2 (Utilities|Casting|CastToGM_RopePuller _returnvalue_2))
  (bind _boxextent (Variables|/Script/Engine.BoxComponent|GetBoxExtent _boxarea))
  (bind (_x _y _z) (Math|Vector|BreakVector _returnvalue_3))
  (bind _y_2 (Math|Vector|BreakVector _boxextent))
  (bind _lightintensity (Variables|/Game/Blueprint/GM_RopePuller.GM_RopePuller_C|GetlightIntensity _asgm_rope_puller))
  (bind _lightintensity_2 (Variables|/Game/Blueprint/GM_RopePuller.GM_RopePuller_C|GetlightIntensity _asgm_rope_puller_2))
  ;[1 1 1] To tweak on spawnrates and amount
  (Utilities|FlowControl|Delay (Variables|Default|GetSpawnDelay))
  (for _index (range 0 (Math|Random|RandomInteger 4))
    (if true ; determine if smth is spawn on this iteration
      (bind _output_get (Variables|Default|SetratioRandom (Math|Random|RandomFloatinRange 0.0 1.0)))
      (Variables|Default|SetrandomSpawnLocation (Math|Vector|MakeVector _x (+ _y (* 5 (Math|Random|RandomFloatinRange (* -100 _y_2) (* 100 _y_2)))) _z))
      (if (< _output_get 0.6) ; Check if spawn Obstacle
        (Game|SpawnActorfromClass "/Game/Blueprint/BP_TestObstacle.BP_TestObstacle_C" (Math|Transform|MakeTransform (Variables|Default|GetrandomSpawnLocation)) "DontSpawnIfColliding" 0 0)
        (else
          ;[0 0.7961 0.9062] WaterDrops
          (if (< (Variables|Default|GetratioRandom) 0.7) ; Check if spawn WaterDrop
            (if (or (> _lightintensity_2 75.0) (< _lightintensity_2 25.0)) ; Need to spawn in danger ?
              ;;[0 0.006305 0.1302] Control (The waterdrop will spawn in the more dangerous zone)
              (if (> _lightintensity_2 5e+01) ; side check
                ;;;[1 1 1] Obscurity
                (Game|SpawnActorfromClass "/Game/Blueprint/BP_WaterDrops.BP_WaterDrops_C" (Math|Transform|MakeTransform (Math|Vector|MakeVector (.X (Math|Vector|BreakVector (Variables|Default|GetrandomSpawnLocation))) (Math|Float|Absolute(Float) (.Y (Math|Vector|BreakVector (Variables|Default|GetrandomSpawnLocation)))) (.Z (Math|Vector|BreakVector (Variables|Default|GetrandomSpawnLocation))))) "Undefined" 0 0)
                (else
                  (Game|SpawnActorfromClass "/Game/Blueprint/BP_WaterDrops.BP_WaterDrops_C" (Math|Transform|MakeTransform (Math|Vector|MakeVector (.X (Math|Vector|BreakVector (Variables|Default|GetrandomSpawnLocation))) (* (Math|Float|Absolute(Float) (.Y (Math|Vector|BreakVector (Variables|Default|GetrandomSpawnLocation)))) -1.0) (.Z (Math|Vector|BreakVector (Variables|Default|GetrandomSpawnLocation))))) "Undefined" 0 0)))
              (else
                ;;[1 1 1] Spawn anywhere randomly
                (Game|SpawnActorfromClass "/Game/Blueprint/BP_WaterDrops.BP_WaterDrops_C" (Math|Transform|MakeTransform (Variables|Default|GetrandomSpawnLocation)) "Undefined" 0 0)))
            (else
              ;[0 1 0.05731] Acid Drops
              (if (< (Variables|Default|GetratioRandom) 0.8) ; Acid Drops
                (if (or (> _lightintensity 75.0) (< _lightintensity 25.0)) ; Need to spawn in danger ?
                  ;;[0 0 0] Control (The waterdrop will spawn in the more dangerous zone)
                  (if (> _lightintensity 5e+01) ; side check
                    ;;;[1 1 1] Obscurity
                    (Game|SpawnActorfromClass "/Game/Blueprint/BP_AcidDrops.BP_AcidDrops_C" (Math|Transform|MakeTransform (Math|Vector|MakeVector (.X (Math|Vector|BreakVector (Variables|Default|GetrandomSpawnLocation))) (* (Math|Float|Absolute(Float) (.Y (Math|Vector|BreakVector (Variables|Default|GetrandomSpawnLocation)))) -1.0) (.Z (Math|Vector|BreakVector (Variables|Default|GetrandomSpawnLocation))))) "Undefined" 0 0)
                    (else
                      (Game|SpawnActorfromClass "/Game/Blueprint/BP_AcidDrops.BP_AcidDrops_C" (Math|Transform|MakeTransform (Math|Vector|MakeVector (.X (Math|Vector|BreakVector (Variables|Default|GetrandomSpawnLocation))) (Math|Float|Absolute(Float) (.Y (Math|Vector|BreakVector (Variables|Default|GetrandomSpawnLocation)))) (.Z (Math|Vector|BreakVector (Variables|Default|GetrandomSpawnLocation))))) "Undefined" 0 0)))
                  (else
                    ;;[1 1 1] Spawn anywhere randomly
                    (Game|SpawnActorfromClass "/Game/Blueprint/BP_AcidDrops.BP_AcidDrops_C" (Math|Transform|MakeTransform (Variables|Default|GetrandomSpawnLocation)) "Undefined" 0 0)))
                (elif (< (Variables|Default|GetratioRandom) 0.95) ; Orbs : \nTrue = default\nFalse = timed orbs
                  ;[1 1 1] Basic orb
                  (Game|SpawnActorfromClass "/Game/Blueprint/BP_NormalOrb.BP_NormalOrb_C" (Math|Transform|MakeTransform (Variables|Default|GetrandomSpawnLocation)) "DontSpawnIfColliding" 0 0)
                  (else
                    ;[1 1 1] Specfic orb depending on light intensity
                    (if (> (Variables|/Game/Blueprint/GM_RopePuller.GM_RopePuller_C|GetlightIntensity (.AsGM%20Rope%20Puller (Utilities|Casting|CastToGM_RopePuller (Game|GetGameMode)))) 5e+01) ; Check light status
                      (Game|SpawnActorfromClass "/Game/Blueprint/BP_ShadowOrb.BP_ShadowOrb_C" (Math|Transform|MakeTransform (Variables|Default|GetrandomSpawnLocation)) "DontSpawnIfColliding" 0 0)
                      (else
                        (Game|SpawnActorfromClass "/Game/Blueprint/BP_LightOrb.BP_LightOrb_C" (Math|Transform|MakeTransform (Variables|Default|GetrandomSpawnLocation)) "DontSpawnIfColliding" 0 0))))))))))))
  (CallFunction|Relay))

(fn ConstructionScript)