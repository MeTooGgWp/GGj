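; Flower actor for the rope-puller game mode that tracks collected petals and routes orbs to the players.
; Adding or removing petals toggles eight preplaced planes, with additions triggering the game mode's win check.
; Basic orbs wait on the flower or go to a random player, while shadow and light orbs charge their matching character.
; Tick swaps the dynamic material's texture by light intensity, and a timeline handles temporary growth.
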(event Custom|unexpectedGrowth
  (params (duration :type Float%20%28single-precision%29))
  (bind _newtrack_0 (Timeline|Growth Play)
    (:Update
      (Transformation|SetActorScale3D (Math|Vector|Lerp(Vector) "1.000000,1.000000,1.000000" "2.000000,2.000000,2.000000" _newtrack_0)))
    (:Finished
      (Utilities|FlowControl|RetriggerableDelay duration)
      (Timeline|Growth Reverse))))

(event EventTick
  (params (DeltaSeconds :type Float%20%28single-precision%29))
  (bind _gamemoderef (Variables|Default|GetgamemodeREF))
  (bind _dynamicmatref (Variables|Default|GetdynamicMatREF))
  (bind _lightintensity (Variables|/Game/Blueprint/GM_RopePuller.GM_RopePuller_C|GetlightIntensity _gamemoderef))
  (bind _returnvalue (< _lightintensity 2e+01))
  (if (or _returnvalue (> _lightintensity 8e+01))
    (if _returnvalue
      (Rendering|Material|SetTextureParameterValue _dynamicmatref "Texture" "/Game/Texture/Flower/T_FlowerDayHOT.T_FlowerDayHOT")
      (else
        (Rendering|Material|SetTextureParameterValue _dynamicmatref "Texture" "/Game/Texture/Flower/T_FlowerNightCOLD.T_FlowerNightCOLD")))
    (else
      (Rendering|Material|SetTextureParameterValue _dynamicmatref "Texture" "/Game/Texture/Flower/T_FlowerBase.T_FlowerBase"))))

(event EventBeginPlay
  (Variables|Default|SetgamemodeREF (.AsGM%20Rope%20Puller (Utilities|Casting|CastToGM_RopePuller (Game|GetGameMode))))
  ;[1 1 1] AWFULL but testing purposes
  (Utilities|Array|Add (Variables|Default|GetpetalsArray) (Variables|Default|Getplane))
  (Utilities|Array|Add (Variables|Default|GetpetalsArray) (Variables|Default|Getplane1))
  (Utilities|Array|Add (Variables|Default|GetpetalsArray) (Variables|Default|Getplane2))
  (Utilities|Array|Add (Variables|Default|GetpetalsArray) (Variables|Default|Getplane3))
  (Utilities|Array|Add (Variables|Default|GetpetalsArray) (Variables|Default|Getplane4))
  (Utilities|Array|Add (Variables|Default|GetpetalsArray) (Variables|Default|Getplane5))
  (Utilities|Array|Add (Variables|Default|GetpetalsArray) (Variables|Default|Getplane6))
  (Utilities|Array|Add (Variables|Default|GetpetalsArray) (Variables|Default|Getplane7))
  (for _array_element (Variables|Default|GetpetalsArray)
    (Rendering|SetVisibility _array_element false false)))

(fn ConstructionScript
  (bind _returnvalue (Rendering|Material|CreateDynamicMaterialInstance "/Game/Material/M_FlowerHead.M_FlowerHead" "None" "None" :!class /Script/Engine.KismetMaterialLibrary))
  (bind _output_get (Variables|Default|SetdynamicMatREF _returnvalue))
  (Rendering|Material|SetMaterial (Variables|Default|GetFlowerBase) 0 _output_get))

(fn AddPetal
  (Development|PrintString "Hello")
  (CallFunction|SpawnPetal)
  (bind _output_get (Variables|Default|SetamountOfPetals (+ (Variables|Default|GetamountOfPetals) 1)))
  (Default|CheckWin (.AsGM%20Rope%20Puller (Utilities|Casting|CastToGM_RopePuller (Game|GetGameMode))) _output_get))

(fn RemovePetal
  (if (> (Variables|Default|GetamountOfPetals) 0)
    (Variables|Default|SetamountOfPetals (- (Variables|Default|GetamountOfPetals) 1))
    (CallFunction|DespawnPetal)))

(fn CollectBasicOrbs
  (if (Variables|Default|GethasOrbsWaiting?)
    ;[1 1 1] randomly assign previous orb to a player
    (Default|AbsorbShard (.AsBP%20Player%20Lutin (Utilities|Casting|CastToBP_PlayerLutin (Game|Player|GetPlayerPawn (Math|Random|RandomInteger 2)))))
    (else
      ;[1 1 1] Assign Orbs to Flower
      (Variables|Default|SethasOrbsWaiting? true))))

(fn CollectShadowOrb
  (bind _returnvalue (Game|Player|GetPlayerPawn 0))
  (bind (_asbp_shadow_player _bsuccess) (Utilities|Casting|CastToBP_ShadowPlayer _returnvalue))
  ;[1 1 1] Determine wich player incarn the shadow character
  (if _bsuccess
    ;[1 1 1] Add charge if there was none
    (Variables|/Game/Blueprint/BP_PlayerLutin.BP_PlayerLutin_C|SethasCharge? _asbp_shadow_player true)
    (else
      (Variables|/Game/Blueprint/BP_PlayerLutin.BP_PlayerLutin_C|SethasCharge? (.AsBP%20Shadow%20Player (Utilities|Casting|CastToBP_ShadowPlayer (Game|Player|GetPlayerPawn 1))) true))))

(fn CollectLightOrb
  (bind _returnvalue (Game|Player|GetPlayerPawn 0))
  (bind (_asbp_light_player _bsuccess) (Utilities|Casting|CastToBP_LightPlayer _returnvalue))
  ;[1 1 1] Determine wich player incarn the light character
  (if _bsuccess
    ;[1 1 1] Add charge if there was none
    (Variables|/Game/Blueprint/BP_PlayerLutin.BP_PlayerLutin_C|SethasCharge? _asbp_light_player true)
    (else
      (Variables|/Game/Blueprint/BP_PlayerLutin.BP_PlayerLutin_C|SethasCharge? (.AsBP%20Light%20Player (Utilities|Casting|CastToBP_LightPlayer (Game|Player|GetPlayerPawn 1))) true))))

(fn SpawnPetal
  (Rendering|SetVisibility (Utilities|Array|Get(acopy) (Variables|Default|GetpetalsArray) (Variables|Default|GetamountOfPetals)) true false))

(fn DespawnPetal
  (Rendering|SetVisibility (Utilities|Array|Get(acopy) (Variables|Default|GetpetalsArray) (Variables|Default|GetamountOfPetals)) false false))