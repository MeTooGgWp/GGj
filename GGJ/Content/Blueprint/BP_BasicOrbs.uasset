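; BP_BasicOrbs is a falling collectible orb that the flower gathers by touch.
; On BeginPlay a Timeline lerps it from its spawn location straight down to world Z zero, simulating a fall without physics, then destroys it when finished.
; An overlap on its sphere component with BP_Flower calls that flower's CollectBasicOrbs and destroys the orb.
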(event OnComponentBeginOverlap(Sphere1)
  (params (OverlappedComponent :type Primitive%20Component%20Object%20Reference) (OtherActor :type Actor%20Object%20Reference) (OtherComp :type Primitive%20Component%20Object%20Reference) (OtherBodyIndex :type Integer) (bFromSweep :type Boolean) (SweepResult :type Hit%20Result%20Structure%20%28by%20ref%29))
  (bind (_asbp_flower _bsuccess) (Utilities|Casting|CastToBP_Flower OtherActor))
  ;[1 1 1] On touch with the flower
  (if _bsuccess
    (Default|CollectBasicOrbs _asbp_flower)
    (Actor|DestroyActor)))

(event EventBeginPlay
  ;[1 1 1] Basic behaviour (simulate falling)
  (Variables|Default|SetinitialSpawnLocation (Transformation|GetActorLocation))
  (bind _newtrack_0 (Timeline|Timeline_0 PlayFromStart)
    (:Update
      (Transformation|SetWorldLocation (Variables|Transformation|GetRootComponent) (Math|Vector|Lerp(Vector) (Variables|Default|GetinitialSpawnLocation) (Math|Vector|MakeVector (.X (Math|Vector|BreakVector (Variables|Default|GetinitialSpawnLocation))) (.Y (Math|Vector|BreakVector (Variables|Default|GetinitialSpawnLocation))) 0.0) _newtrack_0) false false))
    (:Finished
      (Actor|DestroyActor))))

(fn ConstructionScript)